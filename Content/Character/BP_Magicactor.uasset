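; BP_Magicactor is a magic projectile that flies toward a target actor and damages the battle character it hits.
; On BeginPlay or Initialize, it sets its movement velocity once from the target's current location, with no homing.
; Overlapping any BattleCharacter other than its owning character calls the owner's OnDamage with fixed magic power and the victim's defence, then spawns an explosion and destroys the projectile.
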(event `self.ReceiveBeginPlay`
  (bind _targetactor (`self.TargetActor`))
  ;[1 1 1] 初回処理
  (`/Engine/EditorBlueprintResources/StandardMacros.IsValid` _targetactor :!label _label
    (:`Is Valid`
      (set `MovementComponent.Velocity` (`self.GetMoveDirection` (`self.K2_GetActorLocation` _targetactor)) (`self.MyMovement`)))))

(event `Initialize`
  ;[1 1 1] 初回処理
  (goto _label))

(event `self.Collision.OnComponentBeginOverlap`
  (params (OverlappedComponent :type "PrimitiveComponent Object Reference") (OtherActor :type "Actor Object Reference") (OtherComp :type "PrimitiveComponent Object Reference") (OtherBodyIndex :type Integer) (bFromSweep :type Boolean) (SweepResult :type "HitResult Structure (by ref)"))
  (bind _asbattle_character (cast `BattleCharacter` OtherActor))
  (if (!= _asbattle_character (`self.MyCharacter`))
    (bind (_mystatus_myteam _mystatus_equipstate _mystatus_battlestate _mystatus_name _mystatus_maxhp _mystatus_maxsp _mystatus_str _mystatus_def) (break `CharacterStatus` (`BattleCharacter.MyStatus` _asbattle_character)))
    (`CharacterInterface.OnDamage` (`self.MyCharacter`) 10.0 _asbattle_character (`KismetMathLibrary.Conv_IntToDouble` _mystatus_def))
    (`|SpawnActorFromClass` "/Game/Character/BP_Explosion.BP_Explosion_C" (`SceneComponent.K2_GetComponentToWorld` OverlappedComponent) "Undefined" "OverrideRootScale" null null)
    (`self.K2_DestroyActor`)))

(fn `UserConstructionScript`)